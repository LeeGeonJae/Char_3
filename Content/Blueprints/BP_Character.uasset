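; Player character Blueprint with axis-driven movement, mouse look and a Space Bar jump, which dies on touching a "Floor"-tagged actor.
; Movement follows the controller's forward and right vectors, while Turn and LookUp feed controller yaw and pitch.
; A capsule hit on the floor tag fires once, turning the mesh into a physics ragdoll, deactivating CharacterMovement and restarting the level by console command after a short delay.
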(event OnComponentHit(CapsuleComponent)
  (params (HitComponent :type Primitive%20Component%20Object%20Reference) (OtherActor :type Actor%20Object%20Reference) (OtherComp :type Primitive%20Component%20Object%20Reference) (NormalImpulse :type Vector :default "0, 0, 0") (Hit :type Hit%20Result%20Structure%20%28by%20ref%29))
  (bind _mesh (Variables|Character|GetMesh))
  (if (Actor|ActorHasTag OtherActor "Floor")
    (Utilities|FlowControl|DoOnce false
      (:Completed
        (Physics|SetSimulatePhysics _mesh true)
        (Collision|SetCollisionEnabled _mesh "QueryAndPhysics")
        (Components|Activation|SetActive (Variables|Character|GetCharacterMovement) false false)
        (Utilities|FlowControl|Delay 3.0)
        (Development|ExecuteConsoleCommand "restartlevel" 0)))))

(event EventBeginPlay)

(event Collision|EventActorBeginOverlap
  (params (OtherActor :type Actor%20Object%20Reference)))

(event EventTick
  (params (DeltaSeconds :type Float%20%28single-precision%29)))

(event Input|AxisEvents|InputAxisMoveRight
  (params (AxisValue :type Float%20%28single-precision%29))
  (Pawn|Input|AddMovementInput (Transformation|GetActorRightVector (Pawn|GetController)) AxisValue false))

(event Input|AxisEvents|InputAxisMoveForward
  (params (AxisValue :type Float%20%28single-precision%29))
  (Pawn|Input|AddMovementInput (Transformation|GetActorForwardVector (Pawn|GetController)) AxisValue false))

(event Input|AxisEvents|InputAxisTurn
  (params (AxisValue :type Float%20%28single-precision%29))
  ;[1 1 1] 마우스를 콘트롤러 기능을 추가해 회전할 수 있도록
  (Pawn|Input|AddControllerYawInput AxisValue))

(event Input|AxisEvents|InputAxisLookUp
  (params (AxisValue :type Float%20%28single-precision%29))
  ;[1 1 1] 마우스를 콘트롤러 기능을 추가해 회전할 수 있도록
  (Pawn|Input|AddControllerPitchInput AxisValue))

(event Input|KeyboardEvents|SpaceBar
  (params (Key :type Key%20Structure :default "None"))
  (:Pressed
    (Character|Jump)))

(fn ConstructionScript)